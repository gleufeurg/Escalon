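; BP_FadeMesh is a world mesh actor that can fade toward a configurable ending opacity and back.
; The construction script assigns the configured mesh and a dynamic instance of the fade material.
; StartFade plays a timeline whose FadeAmount drives the material's Opacity parameter from 1 toward EndingFloatAmount, and EndFade reverses that timeline to restore it.
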(event EventEndFade
  (bind _fade_amount (Timeline|Timeline Reverse)
    (:Update
      (Rendering|Material|SetScalarParameterValue (Variables|Default|GetDynamicMaterial) "Opacity" (- 1.0 (* _fade_amount (- 1.0 (Variables|Default|GetEndingFloatAmount)))) :!class /Script/Engine.MaterialInstanceDynamic))))

(event EventStartFade
  (bind _fade_amount (Timeline|Timeline Play)
    (:Update
      (Rendering|Material|SetScalarParameterValue (Variables|Default|GetDynamicMaterial) "Opacity" (- 1.0 (* _fade_amount (- 1.0 (Variables|Default|GetEndingFloatAmount)))) :!class /Script/Engine.MaterialInstanceDynamic))))

(fn ConstructionScript
  (Components|StaticMesh|SetStaticMesh (Variables|Default|GetStaticMesh) (Variables|Default|GetMeshToUse))
  (bind _returnvalue (Rendering|Material|CreateDynamicMaterialInstance (Variables|Default|GetFadeMaterial) "None" "None" :!class /Script/Engine.KismetMaterialLibrary))
  (bind _output_get (Variables|Default|SetDynamicMaterial _returnvalue))
  (Rendering|Material|SetMaterial (Variables|Default|GetStaticMesh) 0 _output_get))