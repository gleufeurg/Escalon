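; BPC_Weapon is the parent weapon component that links a weapon to the player's third-person character.
; On BeginPlay it registers itself as the character's weapon, then loads Damage and GaugeGain from its DT_Item data table row.
; Its Attack event forwards the call to the player character's Attack.
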(event Custom|Attack
  (bind _asbp_third_person_character (Utilities|Casting|CastToBP_ThirdPersonCharacter (Game|GetPlayerCharacter 0)))
  (Default|Attack _asbp_third_person_character))

(event EventBeginPlay
  (bind _asbp_third_person_character (Utilities|Casting|CastToBP_ThirdPersonCharacter (Game|GetPlayerCharacter 0)))
  (Variables|/Game/ThirdPerson/Blueprints/BP_ThirdPersonCharacter.BP_ThirdPersonCharacter_C|SetBPC_Weapon _asbp_third_person_character self)
  (bind _returnvalue (Utilities|GetDataTableRow "/Game/Inventory/DT_Item.DT_Item" (.rowname (Variables|Default|GetData)))
    (:then
      (Variables|Default|SetDamage (.damage _returnvalue))
      (Variables|Default|SetGauge%20Gain (.gaugegain _returnvalue)))))