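; Skill component for Arrow Rain, extending a parent skill that supplies the base UseSkill behavior.
; On use, it casts the owner to BP_Player and spawns the NS_ArrowRain Niagara effect above the player's TargetLoc, a targeting method noted as temporary until mouse-aimed casting.
; The BP_ArrowRain actor spawn that passes tick timing, activation count and damage is disconnected, so this graph itself only spawns the visual.
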(event EventBeginPlay
  (|CallParentFunction))

(event EventUseSkill
  (|CallParentFunction)
  ;[0 0 0 0.85] A changer avec le target system via la souris
  ; Le prochain systeme fera en sorte de cast le skill là où la souris est (dans un rayion défini autour du joueur)
  (bind _asbp_third_person_character (Utilities|Casting|CastToBP_Player (Components|GetOwner)))
  ;[1 1 1] New arrow rain
  (Niagara|SpawnSystematLocation "/Game/FX/Effects/ArrowRain/NS_ArrowRain.NS_ArrowRain" (+ (Variables|/Game/Player/Blueprints/BP_Player.BP_Player_C|GetTarget%20Loc _asbp_third_person_character) "0.000000,0.000000,500.000000")))