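; Dash skill component that launches the player character toward its target location, passing through pawns.
; UseSkill calls the parent, turns the character to face TargetLoc, sets capsule Pawn collision to Overlap, then launches it along its forward vector by DashDist.
; Input is disabled during a short fixed Delay, a stand-in for a future animation notify, after which input returns, movement stops and Pawn blocking is restored.
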(event EventBeginPlay
  (|CallParentFunction))

(event EventUseSkill
  (bind _returnvalue (Game|GetPlayerController 0))
  (|CallParentFunction)
  (bind _asbp_third_person_character (Utilities|Casting|CastToBP_ThirdPersonCharacter (Game|GetPlayerCharacter 0)))
  (Transformation|SetActorRotation _asbp_third_person_character (Math|Rotator|MakeRotator (.roll (Math|Rotator|FindLookatRotation (Transformation|GetActorLocation _asbp_third_person_character) (Variables|/Game/Player/Blueprints/BP_ThirdPersonCharacter.BP_ThirdPersonCharacter_C|GetTarget%20Loc _asbp_third_person_character))) 0.0 (.yaw (Math|Rotator|FindLookatRotation (Transformation|GetActorLocation _asbp_third_person_character) (Variables|/Game/Player/Blueprints/BP_ThirdPersonCharacter.BP_ThirdPersonCharacter_C|GetTarget%20Loc _asbp_third_person_character)))))
  ;[0.2188 0.6541 1 0.85] The Player Dash through enemies
  (Collision|SetCollisionResponsetoChannel (Variables|/Script/Engine.Character|GetCapsuleComponent _asbp_third_person_character) "ECC_Pawn" "ECR_Overlap")
  (Character|LaunchCharacter _asbp_third_person_character (* (Transformation|GetActorForwardVector _asbp_third_person_character) (Variables|Default|GetDash%20Dist)) true true)
  ;[0.08333 0.08333 0.08333 0.85] The Player can't act during the dash
  ; When there will be an anim for the dash, this will be handled by an
  ; Event Notify
  (Input|DisableInput _asbp_third_person_character _returnvalue)
  (Utilities|FlowControl|Delay 0.25)
  ;[0.08854 0.08854 0.08854 0.85] Reset all cahngement made to the player during the dash (Collisions, Inputs...)
  (Input|EnableInput _asbp_third_person_character _returnvalue)
  (Components|Movement|StopMovementImmediately (Variables|/Script/Engine.Character|GetCharacterMovement _asbp_third_person_character))
  (Collision|SetCollisionResponsetoChannel (Variables|/Script/Engine.Character|GetCapsuleComponent _asbp_third_person_character) "ECC_Pawn" "ECR_Block"))