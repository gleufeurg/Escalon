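; Dash skill component that launches the player toward their target location and through enemies, damaging those hit.
; UseSkill turns the character, sets pawn collision to overlap, launches it forward, disables input and starts Niagara trail and speed-line effects.
; EndSkill restores input and collision, then, if an enemy was hit, plays a slash effect with brief time-dilation hit-stop and applies damage to the recorded enemies.
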(event EventBeginPlay
  (|CallParentFunction))

(event EventUseSkill
  (|CallParentFunction)
  (bind _asbp_third_person_character (Utilities|Casting|CastToBP_ThirdPersonCharacter (Game|GetPlayerCharacter 0)))
  (Transformation|SetActorRotation _asbp_third_person_character (Math|Rotator|MakeRotator (.roll (Math|Rotator|FindLookatRotation (Transformation|GetActorLocation _asbp_third_person_character) (Variables|/Game/Player/Blueprints/BP_ThirdPersonCharacter.BP_ThirdPersonCharacter_C|GetTarget%20Loc _asbp_third_person_character))) 0.0 (.yaw (Math|Rotator|FindLookatRotation (Transformation|GetActorLocation _asbp_third_person_character) (Variables|/Game/Player/Blueprints/BP_ThirdPersonCharacter.BP_ThirdPersonCharacter_C|GetTarget%20Loc _asbp_third_person_character)))))
  ;[0.2188 0.6541 1 0.85] The Player Dash through enemies
  (Collision|SetCollisionResponsetoChannel (Variables|/Script/Engine.Character|GetCapsuleComponent _asbp_third_person_character) "ECC_Pawn" "ECR_Overlap")
  (Components|Movement|StopMovementImmediately (Variables|/Script/Engine.Character|GetCharacterMovement _asbp_third_person_character))
  (Character|LaunchCharacter _asbp_third_person_character (* (Transformation|GetActorForwardVector _asbp_third_person_character) (Variables|Default|GetDash%20Dist)) true true)
  ;[0.08333 0.08333 0.08333 0.85] The Player can't act during the dash
  ; When there will be an anim for the dash, this will be handled by an
  ; Event Notify
  (Input|DisableInput _asbp_third_person_character (Game|GetPlayerController 0))
  (Niagara|SpawnSystemAttached "/Game/FX/Effects/Dash/NS_Dash.NS_Dash" (Variables|/Game/Player/Blueprints/BP_ThirdPersonCharacter.BP_ThirdPersonCharacter_C|GetPickUpArrow _asbp_third_person_character) "None" (.location (Transformation|GetActorTransform _asbp_third_person_character)) (.rotation (Transformation|GetActorTransform _asbp_third_person_character)) "KeepRelativeOffset" false)
  (Components|Activation|Activate (Variables|/Game/Player/Blueprints/BP_ThirdPersonCharacter.BP_ThirdPersonCharacter_C|GetNS_SpeedLines _asbp_third_person_character) true))

(event EventEndSkill
  ;[0.08854 0.08854 0.08854 0.85] Reset all cahngement made to the player during the dash (Collisions, Inputs...)
  (|CallParentFunction)
  (bind _asbp_third_person_character (Utilities|Casting|CastToBP_ThirdPersonCharacter (Game|GetPlayerCharacter 0)))
  (Input|EnableInput _asbp_third_person_character (Game|GetPlayerController 0))
  (Components|Movement|StopMovementImmediately (Variables|/Script/Engine.Character|GetCharacterMovement _asbp_third_person_character))
  (Collision|SetCollisionResponsetoChannel (Variables|/Script/Engine.Character|GetCapsuleComponent _asbp_third_person_character) "ECC_Pawn" "ECR_Block")
  (Utilities|Time|SetGlobalTimeDilation 1.0)
  (if (Variables|Default|Gethitted%20enemy)
    (Components|Activation|Activate (Variables|/Game/Player/Blueprints/BP_ThirdPersonCharacter.BP_ThirdPersonCharacter_C|GetNS_DashSlash _asbp_third_person_character) true)
    (Utilities|Time|SetGlobalTimeDilation 0.1)
    (Utilities|FlowControl|Delay 0.07)
    (for _array_element (Variables|Default|GetEnemies_hitted)
      (Class|IDamageable|TakeDamage(Message) _array_element (Variables|Default|GetDamage))
      (Utilities|FlowControl|Delay 0.03)
      (Utilities|Time|SetGlobalTimeDilation 1.0)
      (Utilities|Array|Clear (Variables|Default|GetEnemies_hitted)))))