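; BPC_Skill is a parent skill component that gives the player character a skill paid for with gauge points.
; On BeginPlay it adds its input mapping context to the first player controller and registers itself as the BPCSkill of BP_ThirdPersonCharacter.
; UseSkill deducts Cost through the character's LoseGaugePoints, with no affordability check or skill effect at this level.
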(event Custom|Use%20Skill
  (bind _asbp_third_person_character (Utilities|Casting|CastToBP_ThirdPersonCharacter (Game|GetPlayerCharacter 0)))
  (Default|LoseGaugePoints _asbp_third_person_character (Variables|Default|GetCost)))

(event EventBeginPlay
  (Input|AddMappingContext (PlayerController|LocalPlayerSubsystems|GetEnhancedInputLocalPlayerSubsystem (Game|GetPlayerController 0)) (Variables|Default|GetMapping%20Context) 0 "(bIgnoreAllPressedKeysUntilRelease=True,bForceImmediately=False)")
  (bind _asbp_third_person_character (Utilities|Casting|CastToBP_ThirdPersonCharacter (Game|GetPlayerCharacter 0)))
  (Variables|/Game/ThirdPerson/Blueprints/BP_ThirdPersonCharacter.BP_ThirdPersonCharacter_C|SetBPC_Skill _asbp_third_person_character self))