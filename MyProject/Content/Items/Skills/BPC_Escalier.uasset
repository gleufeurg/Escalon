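; Skill component that spawns an Escalier (staircase) actor in front of the player.
; UseSkill places the actor 1000 units along the follow camera's forward vector, aligned to the camera manager's rotation and adjusted for collisions but always spawned.
; It then deducts the skill's Cost from the third-person character's gauge through LoseGaugePoints, with no check on the available points in this graph.
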(event EventBeginPlay
  (|CallParentFunction))

(event EventUseSkill
  (bind _asbp_third_person_character (Utilities|Casting|CastToBP_ThirdPersonCharacter (Game|GetPlayerCharacter 0)))
  (Game|SpawnActorfromClass "/Game/Items/Skills/Escalier.Escalier_C" (Math|Transform|MakeTransform (+ (Transformation|GetWorldLocation (Variables|/Game/ThirdPerson/Blueprints/BP_ThirdPersonCharacter.BP_ThirdPersonCharacter_C|GetFollowCamera _asbp_third_person_character)) (* (Math|Vector|GetForwardVector (Variables|/Game/ThirdPerson/Blueprints/BP_ThirdPersonCharacter.BP_ThirdPersonCharacter_C|GetFollowCamera _asbp_third_person_character)) (Math|Float|MakeLiteralFloat 1e+03))) (Camera|GetCameraRotation (Game|GetPlayerCameraManager 0)) "1.000000,1.000000,1.000000") "AdjustIfPossibleButAlwaysSpawn" "MultiplyWithRoot" 0 0)
  (bind _asbp_third_person_character_2 (Utilities|Casting|CastToBP_ThirdPersonCharacter (Game|GetPlayerCharacter 0)))
  (Default|LoseGaugePoints _asbp_third_person_character_2 (Variables|Default|GetCost)))