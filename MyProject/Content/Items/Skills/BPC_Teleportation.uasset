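; BPC_Teleportation is a skill component that blinks the player forward by a dash distance.
; On UseSkill, it runs the parent logic, gets the BP_Player and line-traces along the actor's forward vector on the Visibility channel.
; It teleports the player to the end point without sweeping only if the trace hits nothing, so a blocked path means no movement rather than a shortened dash.
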(event EventBeginPlay
  (|CallParentFunction))

(event EventUseSkill
  (|CallParentFunction)
  (bind _asbp_third_person_character (Utilities|Casting|CastToBP_Player (Game|GetPlayerCharacter 0)))
  (bind _returnvalue (Collision|LineTraceByChannel (Transformation|GetActorLocation _asbp_third_person_character) (+ (Transformation|GetActorLocation _asbp_third_person_character) (* (Transformation|GetActorForwardVector _asbp_third_person_character) (Variables|Default|GetDash%20Dist))) "TraceTypeQuery1" false 0 "None"))
  (if (not _returnvalue)
    (Transformation|SetActorLocation _asbp_third_person_character (+ (Transformation|GetActorLocation _asbp_third_person_character) (* (Transformation|GetActorForwardVector _asbp_third_person_character) (Variables|Default|GetDash%20Dist))) false true)))