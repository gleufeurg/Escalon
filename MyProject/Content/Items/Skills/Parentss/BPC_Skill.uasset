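; BPC_Skill is a parent skill component that handles the gauge cost of using a skill.
; On BeginPlay it looks up its row in DT_Item by Data.RowName and caches the SkillCost.
; UseSkill deducts that cost from the first player's BP_ThirdPersonCharacter gauge points, then calls RingModifier on each of the character's ring components.
; CancelSkill is an empty event.
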(event Custom|Use%20Skill
  (bind _asbp_third_person_character (Utilities|Casting|CastToBP_ThirdPersonCharacter (Game|GetPlayerCharacter 0)))
  (Default|LoseGaugePoints _asbp_third_person_character (Variables|Default|GetCost))
  (for _array_element (Variables|/Game/ThirdPerson/Blueprints/BP_ThirdPersonCharacter.BP_ThirdPersonCharacter_C|GetBPC_Rings _asbp_third_person_character)
    (Default|RingModifier _array_element)))

(event Custom|Cancel%20Skill)

(event EventBeginPlay
  (bind _returnvalue (Utilities|GetDataTableRow "/Game/Inventory/DT_Item.DT_Item" (.rowname (Variables|Default|GetData)))
    (:then
      (Variables|Default|SetCost (.SkillCost (Utilities|Struct|BreakF_Item _returnvalue))))))