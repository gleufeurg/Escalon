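; BPC_SmashWave is a skill component that spawns an Escalier actor for the player character at a gauge cost.
; UseSkill casts player 0 to BP_ThirdPersonCharacter and passes its capsule, that capsule's relative rotation and SpawnDist to Target for a spawn location and rotation.
; It spawns the actor there, adjusting for collisions but always spawning, then deducts Cost through LoseGaugePoints with no gauge check here.
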(event EventBeginPlay
  (|CallParentFunction))

(event EventUseSkill
  (bind _asbp_third_person_character (Utilities|Casting|CastToBP_ThirdPersonCharacter (Game|GetPlayerCharacter 0)))
  (bind (_location _rotation) (CallFunction|Target (Variables|/Script/Engine.Character|GetCapsuleComponent _asbp_third_person_character) (Variables|Default|GetSpawnDist) (Variables|/Script/Engine.SceneComponent|GetRelativeRotation (Variables|/Script/Engine.Character|GetCapsuleComponent _asbp_third_person_character))))
  (Game|SpawnActorfromClass "/Game/Items/Skills/Escalier.Escalier_C" (Math|Transform|MakeTransform _location _rotation "1.000000,1.000000,1.000000") "AdjustIfPossibleButAlwaysSpawn" "MultiplyWithRoot" 0 0)
  (Default|LoseGaugePoints _asbp_third_person_character (Variables|Default|GetCost)))