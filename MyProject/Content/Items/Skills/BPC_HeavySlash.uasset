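; Skill component that gives BP_ThirdPersonCharacter a heavy slash attack dealing its own damage to enemies.
; UseSkill turns off the character's normal weapon damage and binds an overlap handler to the weapon mesh.
; While bound, each overlap with a BP_Enemy sends it TakeDamageMessage with the skill's Damage value.
; EndHeavySlash unbinds the handler and re-enables normal weapon damage; the Unbind function is an empty stub.
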(event Custom|End%20Heavy%20Slash
  (bind _asbp_third_person_character (Utilities|Casting|CastToBP_ThirdPersonCharacter (Components|GetOwner)))
  (Collision|UnbindEventfromOnComponentBeginOverlap (Variables|/Game/Player/Blueprints/BP_ThirdPersonCharacter.BP_ThirdPersonCharacter_C|GetWeaponMesh _asbp_third_person_character) (delegate Custom|Weapon%20Overlap))
  (Variables|/Game/Player/Blueprints/BP_ThirdPersonCharacter.BP_ThirdPersonCharacter_C|SetWeaponInflictDamage _asbp_third_person_character true))

(event Custom|Weapon%20Overlap
  (params (OverlappedComponent :type Primitive%20Component%20Object%20Reference) (OtherActor :type Actor%20Object%20Reference) (OtherComp :type Primitive%20Component%20Object%20Reference) (OtherBodyIndex :type Integer) (bFromSweep :type Boolean) (SweepResult :type Hit%20Result%20Structure%20%28by%20ref%29))
  (bind _asbp_enemy (Utilities|Casting|CastToBP_Enemy OtherActor))
  (Class|IDamageable|TakeDamage(Message) _asbp_enemy (Variables|Default|GetDamage)))

(event EventBeginPlay
  (|CallParentFunction))

(event EventUseSkill
  (bind _asbp_third_person_character (Utilities|Casting|CastToBP_ThirdPersonCharacter (Components|GetOwner)))
  (Variables|/Game/Player/Blueprints/BP_ThirdPersonCharacter.BP_ThirdPersonCharacter_C|SetWeaponInflictDamage _asbp_third_person_character false)
  (Collision|AssignOnComponentBeginOverlap (Variables|/Game/Player/Blueprints/BP_ThirdPersonCharacter.BP_ThirdPersonCharacter_C|GetWeaponMesh _asbp_third_person_character) (delegate Custom|Weapon%20Overlap)))

(fn Unbind)