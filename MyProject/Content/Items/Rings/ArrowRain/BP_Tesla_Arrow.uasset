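; BP_Tesla_Arrow is an arrow actor that forms a damaging electric channel with another Tesla arrow.
; On BeginPlay it links to the second-to-last Tesla arrow in the world's actor list, spawning a Niagara beam toward it plus sparkles.
; Each Tick, a multi sphere trace along that link damages enemies it hits and raises their gauge.
; Debug trace drawing and index printing remain active.
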(event EventBeginPlay
  (bind _returnvalue (Transformation|GetActorLocation))
  (bind _outactors (Actor|GetAllActorsOfClass "BP_Tesla_Arrow_C"))
  (if (not (< (Utilities|Array|Length _outactors) 2))
    (bind _output_get (Variables|Default|SetLinkedTesla (Utilities|Array|Get(acopy) _outactors (- (Utilities|Array|Length _outactors) 2))))
    (bind _returnvalue_2 (Niagara|SpawnSystematLocation "/Game/FX/Effects/ArrowRain/NS_TeslaChannel.NS_TeslaChannel" _returnvalue))
    (Effects|Components|ParticleSystem|SetVectorParameter _returnvalue_2 "End_Loc" (Transformation|GetActorLocation _output_get))
    (Niagara|SpawnSystematLocation "/Game/FX/Effects/ArrowRain/NS_Sparkles.NS_Sparkles" _returnvalue)
    (Niagara|SpawnSystematLocation "/Game/FX/Effects/ArrowRain/NS_Sparkles.NS_Sparkles" _returnvalue)))

(event EventTick
  (params (DeltaSeconds :type Float%20%28single-precision%29))
  (bind _linkedtesla (Variables|Default|GetLinkedTesla))
  (Utilities|IsValid _linkedtesla
    (:Is%20Valid
      (bind _outhits (Collision|MultiSphereTraceByChannel (Transformation|GetActorLocation) (Transformation|GetActorLocation _linkedtesla) (Variables|Default|GetChannelRadius) "TraceTypeQuery1" false 0 "ForOneFrame" true "(R=1.000000,G=0.000000,B=0.000000,A=1.000000)" "(R=0.000000,G=1.000000,B=0.000000,A=1.000000)" 1e+02))
      (for (_array_element _array_index) _outhits
        (bind _asbp_enemy_base (Utilities|Casting|CastToBP_Enemy_Base (.HitActor (Collision|BreakHitResult _array_element))))
        (Default|TakeDamage _asbp_enemy_base 1.0 1.0)
        (Development|PrintString (Utilities|String|ToString(Integer) _array_index))))))

(fn ConstructionScript)