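; BPC_Keen is a Dash ring item component that gives the player body damage.
; Its passive modifier looks up its row in DT_Item and adds that row's damage to the Dash damage.
; The active modifier copies the Dash damage into BP_Player's BodyDamage, and the reset event sets it back to zero.
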(event EventBeginPlay
  (|CallParentFunction))

(event EventModifyPassives
  (params (BPC_Skill :type BPC%20Skill%20Object%20Reference))
  (bind _dash (Variables|Default|GetDash))
  (bind _returnvalue (Utilities|GetDataTableRow "/Game/Inventory/DT_Item.DT_Item" (.rowname (Variables|Default|GetData)))
    (:then
      (Variables|/Game/Items/Skills/Parents/BPC_Skill.BPC_Skill_C|SetDamage _dash (+ (.Damage (Utilities|Struct|BreakF_Item _returnvalue)) (Variables|/Game/Items/Skills/Parents/BPC_Skill.BPC_Skill_C|GetDamage _dash))))))

(event EventModifyPlayerActive
  (bind _asbp_player (Utilities|Casting|CastToBP_Player (Components|GetOwner)))
  (Variables|/Game/Player/Blueprints/BP_Player.BP_Player_C|SetBodyDamage _asbp_player (Variables|/Game/Items/Skills/Parents/BPC_Skill.BPC_Skill_C|GetDamage (Variables|Default|GetDash))))

(event EventResetModifiers
  (bind _asbp_player (Utilities|Casting|CastToBP_Player (Components|GetOwner)))
  (Variables|/Game/Player/Blueprints/BP_Player.BP_Player_C|SetBodyDamage _asbp_player 0.0))