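; BPC_Keen is a ring item component that modifies the owning third-person character's body damage.
; When the player modifier activates, it looks up its row in DT_Item and sets the character's BodyDamage to that row's Damage value.
; Resetting modifiers sets BodyDamage back to zero, overwriting the value rather than adding or subtracting.
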(event EventBeginPlay
  (|CallParentFunction))

(event EventModifyPlayerActive
  (bind _asbp_third_person_character (Utilities|Casting|CastToBP_ThirdPersonCharacter (Components|GetOwner)))
  (bind _returnvalue (Utilities|GetDataTableRow "/Game/Inventory/DT_Item.DT_Item" (.rowname (Variables|Default|GetData)))
    (:then
      (Variables|/Game/Player/Blueprints/BP_ThirdPersonCharacter.BP_ThirdPersonCharacter_C|SetBodyDamage _asbp_third_person_character (.Damage (Utilities|Struct|BreakF_Item _returnvalue))))))

(event EventResetModifiers
  (bind _asbp_third_person_character (Utilities|Casting|CastToBP_ThirdPersonCharacter (Components|GetOwner)))
  (Variables|/Game/Player/Blueprints/BP_ThirdPersonCharacter.BP_ThirdPersonCharacter_C|SetBodyDamage _asbp_third_person_character 0.0))