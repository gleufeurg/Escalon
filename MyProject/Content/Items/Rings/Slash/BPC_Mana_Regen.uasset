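; Ring item component that restores the player's gauge points when their Heavy Slash deals damage.
; On BeginPlay it casts its owner to BP_Player, loops the Skills array and binds RegenMana to the slash damage event of BPC_HeavySlash.
; RegenMana grants PointsGained gauge points and prints a debug string, regardless of which actor was hit.
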(event Custom|RegenMana
  (params (ActorHitted :type BP%20Enemy%20Base%20Object%20Reference))
  (Default|GainGaugePoints (Variables|Default|GetAs%20BP%20Player) (Variables|Default|GetPoints%20Gained))
  (Development|PrintString "Regen mana (beacoup)"))

(event EventBeginPlay
  (|CallParentFunction)
  (bind _asbp_player (Utilities|Casting|CastToBP_Player (Components|GetOwner)))
  (bind _output_get (Variables|Default|SetAs%20BP%20Player _asbp_player))
  (for _array_element (Variables|/Game/Player/Blueprints/BP_Player.BP_Player_C|GetSkills _output_get)
    (bind _asbpc_heavy_slash (Utilities|Casting|CastToBPC_HeavySlash _array_element))
    (EventDispatchers|BindEventtoSlashDamage _asbpc_heavy_slash (delegate Custom|RegenMana))))

(event EventTick
  (params (DeltaSeconds :type Float%20%28single-precision%29)))