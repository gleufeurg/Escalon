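; BPC_VivacityBuff is a timed buff component that boosts the player's attack speed and walk speed.
; On BeginPlay it multiplies both stats on BP_Player (player character 0) and starts a countdown from BuffDuration.
; Tick runs a Cooldown/Ended state switch that, once time expires, divides the same multipliers back out and destroys the component.
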(event Custom|Effect
  (bind _asbp_third_person_character (Utilities|Casting|CastToBP_Player (Game|GetPlayerCharacter 0)))
  ;[0.3657 1 0.2611 0.85] Set Buffs
  (Variables|/Game/Player/Blueprints/BP_Player.BP_Player_C|SetAttack%20Speed%20Multiplier _asbp_third_person_character (* (Variables|/Game/Player/Blueprints/BP_Player.BP_Player_C|GetAttack%20Speed%20Multiplier _asbp_third_person_character) (Variables|Default|GetAttack%20Speed%20Multiplier)))
  (Variables|/Script/Engine.CharacterMovementComponent|SetMaxWalkSpeed (Variables|/Script/Engine.Character|GetCharacterMovement _asbp_third_person_character) (* (Variables|/Script/Engine.CharacterMovementComponent|GetMaxWalkSpeed (Variables|/Script/Engine.Character|GetCharacterMovement _asbp_third_person_character)) (Variables|Default|GetSpeed%20Multiplier)))
  (Variables|Default|SetBuff%20Timer "NewEnumerator0"))

(event Custom|EffectEnd
  (bind _asbp_third_person_character (Utilities|Casting|CastToBP_Player (Game|GetPlayerCharacter 0)))
  (Variables|/Game/Player/Blueprints/BP_Player.BP_Player_C|SetAttack%20Speed%20Multiplier _asbp_third_person_character (/ (Variables|/Game/Player/Blueprints/BP_Player.BP_Player_C|GetAttack%20Speed%20Multiplier _asbp_third_person_character) (Variables|Default|GetAttack%20Speed%20Multiplier)))
  (Variables|/Script/Engine.CharacterMovementComponent|SetMaxWalkSpeed (Variables|/Script/Engine.Character|GetCharacterMovement _asbp_third_person_character) (/ (Variables|/Script/Engine.CharacterMovementComponent|GetMaxWalkSpeed (Variables|/Script/Engine.Character|GetCharacterMovement _asbp_third_person_character)) (Variables|Default|GetSpeed%20Multiplier)))
  (Components|DestroyComponent))

(event EventTick
  (params (DeltaSeconds :type Float%20%28single-precision%29))
  (switch Utilities|FlowControl|Switch|SwitchonETimerState (Variables|Default|GetBuff%20Timer)
    (:NewEnumerator0
      (bind _output_get (Variables|Default|SetCooldown%20Time (- (Variables|Default|GetCooldown%20Time) (Utilities|Time|GetWorldDeltaSeconds))))
      (if (<= _output_get 0.0)
        (Variables|Default|SetBuff%20Timer "NewEnumerator1")))
    (:NewEnumerator1
      (CallFunction|EffectEnd))))

(event EventBeginPlay
  (Variables|Default|SetCooldown%20Time (Variables|Default|GetBuff%20Duration))
  (CallFunction|Effect))