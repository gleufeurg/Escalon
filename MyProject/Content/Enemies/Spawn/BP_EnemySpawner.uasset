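; BP_EnemySpawner is a placeable spawner that creates a preset list of enemies on BeginPlay when Spawn is enabled.
; Each enemy spawns at a random XY offset around the spawner and registers with BP_EnemiesManager.
; It takes the spawner's or its own team, joins that manager array, and receives a Modifier component.
; AddToTeam maps teams to manager arrays, though Alpha currently routes into Charlie.
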(event EventBeginPlay
  (bind _returnvalue (Transformation|GetActorTransform))
  (bind _spawnoffset (Variables|Spawn|GetSpawnOffset))
  (bind _returnvalue_2 (* _spawnoffset -1.0))
  (if (Variables|Spawn|GetSpawn)
    (switch Utilities|FlowControl|Switch|SwitchonE_SpawnMode (Variables|Spawn|GetSpawnMode)
      (:NewEnumerator0
        (bind _returnvalue_3 (Actor|GetActorOfClass "/Game/Enemies/Parent/BP_EnemiesManager.BP_EnemiesManager_C"))
        (Variables|Default|SetManager _returnvalue_3)
        (for _array_element (Variables|Spawn|GetEnemiesToSpawn)
          (bind _returnvalue_4 (Game|SpawnActorfromClass (.class _array_element) (Math|Transform|MakeTransform (Math|Vector|MakeVector (+ (Math|Random|RandomFloatinRange _returnvalue_2 _spawnoffset) (.x (.location _returnvalue))) (+ (Math|Random|RandomFloatinRange _returnvalue_2 _spawnoffset) (.y (.location _returnvalue))) (.z (.location _returnvalue))) (.rotation _returnvalue)) "AdjustIfPossibleButAlwaysSpawn" "MultiplyWithRoot" 0 0))
          (Utilities|Array|Add (Variables|/Game/Enemies/Parent/BP_EnemiesManager.BP_EnemiesManager_C|GetEnemies_allive (Variables|Default|GetManager)) _returnvalue_4)
          (if (.sameteam _array_element)
            (bind _output_get (Variables|/Game/Enemies/Parent/BP_Enemy_Base.BP_Enemy_Base_C|SetTeam _returnvalue_4 (Variables|Spawn|GetTeam)))
            (CallFunction|AddtoTeam _output_get _returnvalue_4)
            (else
              (bind _output_get_2 (Variables|/Game/Enemies/Parent/BP_Enemy_Base.BP_Enemy_Base_C|SetTeam _returnvalue_4 (.team _array_element)))
              (CallFunction|AddtoTeam _output_get_2 _returnvalue_4)))
          (bind _returnvalue_5 (Game|AddComponentbyClass _returnvalue_4 (.modifier _array_element)))
          (Variables|/Game/Enemies/Parent/BP_Enemy_Base.BP_Enemy_Base_C|SetModifier _returnvalue_4 _returnvalue_5))))))

(fn ConstructionScript)

(fn AddtoTeam
  (params (Selection :type E_Team%20Enum :default "NewEnumerator0") (Enemy :type BP%20Enemy%20Base%20Object%20Reference))
  (bind _manager (Variables|Default|GetManager))
  (switch Utilities|FlowControl|Switch|SwitchonE_Team Selection
    (:NewEnumerator0
      (Utilities|Array|Add (Variables|/Game/Enemies/Parent/BP_EnemiesManager.BP_EnemiesManager_C|GetCharlie _manager) Enemy))
    (:NewEnumerator1
      (Utilities|Array|Add (Variables|/Game/Enemies/Parent/BP_EnemiesManager.BP_EnemiesManager_C|GetBravo _manager) Enemy))
    (:NewEnumerator2
      (Utilities|Array|Add (Variables|/Game/Enemies/Parent/BP_EnemiesManager.BP_EnemiesManager_C|GetCharlie _manager) Enemy))
    (:NewEnumerator3
      (Utilities|Array|Add (Variables|/Game/Enemies/Parent/BP_EnemiesManager.BP_EnemiesManager_C|GetDelta _manager) Enemy))
    (:NewEnumerator4
      (Utilities|Array|Add (Variables|/Game/Enemies/Parent/BP_EnemiesManager.BP_EnemiesManager_C|GetEcho _manager) Enemy))
    (:NewEnumerator5
      (Utilities|Array|Add (Variables|/Game/Enemies/Parent/BP_EnemiesManager.BP_EnemiesManager_C|GetFoxTrot _manager) Enemy))
    (:NewEnumerator6
      (Utilities|Array|Add (Variables|/Game/Enemies/Parent/BP_EnemiesManager.BP_EnemiesManager_C|GetGolf _manager) Enemy))))