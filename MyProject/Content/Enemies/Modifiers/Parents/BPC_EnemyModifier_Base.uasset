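; Base actor component for enemy modifiers, attached to BP_Enemy_Base actors.
; On BeginPlay it finds the BP_EnemiesManager, casts its owner to the enemy base class, and caches that manager, owner and the owner's team fetched from the manager.
; Modifier_Activate is an empty event, apparently left for child modifiers to implement.
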(event Custom|Modifier_Activate)

(event EventBeginPlay
  (bind _returnvalue (Actor|GetActorOfClass "/Game/Enemies/Parent/BP_EnemiesManager.BP_EnemiesManager_C"))
  (Variables|Refs|SetManager _returnvalue)
  (bind _asbp_enemy_base (Utilities|Casting|CastToBP_Enemy_Base (Components|GetOwner)))
  (bind _output_get (Variables|Refs|SetOwner _asbp_enemy_base))
  (Variables|Team|SetETeam (Variables|/Game/Enemies/Parent/BP_Enemy_Base.BP_Enemy_Base_C|GetTeam _output_get))
  (bind _array (Default|GetTeam (Variables|Refs|GetManager) (Variables|Team|GetETeam)))
  (Variables|Team|SetTeam _array))