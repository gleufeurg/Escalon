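; Enemy modifier component that periodically resurrects a dead teammate while its owner is alive.
; On BeginPlay it starts a looping timer at the modifier cooldown, which triggers the ModifierActivate event on top of the parent modifier's logic.
; Each activation resets the first Team member with no health left and teleports it to a random XY offset around the owner, reviving at most one per cycle.
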(event EventBeginPlay
  (|CallParentFunction)
  (Utilities|Time|SetTimerbyEvent (delegate EventModifierActivate) (Variables|Default|GetModifierCooldown) true))

(event EventModifierActivate
  (bind _owner (Variables|Default|GetOwner))
  (bind _spawnoffset (Variables|Modifier|GetSpawnOffset))
  (bind _returnvalue (Transformation|GetActorLocation _owner))
  (bind _returnvalue_2 (* _spawnoffset -1.0))
  (|CallParentFunction)
  (if (not (<= (Variables|/Game/Enemies/Parent/BP_Enemy_Base.BP_Enemy_Base_C|GetHealth (Variables|Default|GetOwner)) 0.0))
    (bind (_array_element _array_index) (Utilities|Array|ForEachLoopwithBreak (Variables|Default|GetTeam) :!label _label)
      (:LoopBody
        (if (<= (Variables|/Game/Enemies/Parent/BP_Enemy_Base.BP_Enemy_Base_C|GetHealth _array_element) 0.0)
          (Default|Reset (Utilities|Array|Get(acopy) (Variables|Default|GetTeam) _array_index))
          (Transformation|SetActorLocation (Utilities|Array|Get(acopy) (Variables|Default|GetTeam) _array_index) (Math|Vector|MakeVector (+ (.x _returnvalue) (Math|Random|RandomFloatinRange _returnvalue_2 _spawnoffset)) (+ (.y _returnvalue) (Math|Random|RandomFloatinRange _returnvalue_2 _spawnoffset)) (.z _returnvalue)) false true)
          (goto _label Break))))))