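; BP_EnemyMelee is a melee enemy Blueprint that performs attacks through a separately spawned attack actor.
; Attack spawns AttackActor at the enemy's transform, stores it in AttackRef and, if it is a BP_MeleeAttack, sets its Damage to zero.
; BeginPlay binds AttackEnd to OnHitboxEnd, so the attack actor is destroyed when that event fires.
; The construction script only runs the parent's.
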(event Custom|AttackEnd
  (Actor|DestroyActor (Variables|Default|GetAttackRef)))

(event EventBeginPlay
  (EventDispatchers|BindEventtoOnHitboxEnd (delegate Custom|AttackEnd)))

(event EventAttack
  (bind _returnvalue (Game|SpawnActorfromClass (Variables|Default|GetAttackActor) (Transformation|GetActorTransform) "AlwaysSpawn" "MultiplyWithRoot" 0 0))
  (bind _output_get (Variables|Default|SetAttackRef _returnvalue))
  (bind _asbp_melee_attack (Utilities|Casting|CastToBP_MeleeAttack _output_get))
  (Variables|/Game/Enemies/Melee/BP_MeleeAttack.BP_MeleeAttack_C|SetDamage _asbp_melee_attack 0.0))

(fn ConstructionScript
  (|CallParentFunction))