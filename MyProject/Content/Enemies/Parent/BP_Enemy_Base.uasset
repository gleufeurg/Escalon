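; Base enemy character Blueprint holding health, movement speed tiers, combat ranges and patrol route.
; TakeDamage subtracts health, grants player gauge points, and triggers randomly offset damage text, camera shake, impact Niagara effect and time-dilation hit stop.
; Die teleports the enemy to BP_EnemiesManager instead of destroying it, while Reset restores health and speed, with both updating the manager's alive and dead lists like a pool.
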(event Custom|Die
  (bind _self self)
  (bind _manager (Variables|Default|GetManager))
  (Utilities|Array|Add (Variables|/Game/Enemies/Parent/BP_EnemiesManager.BP_EnemiesManager_C|GetEnemies_dead _manager) _self)
  (Utilities|Array|RemoveItem (Variables|/Game/Enemies/Parent/BP_EnemiesManager.BP_EnemiesManager_C|GetEnemies_allive _manager) _self)
  (Transformation|SetActorLocation _self (Transformation|GetActorLocation (Variables|Default|GetManager)) false true))

(event EventBeginPlay
  (bind _returnvalue (Actor|GetActorOfClass "/Game/Enemies/Parent/BP_EnemiesManager.BP_EnemiesManager_C"))
  (Variables|Default|SetManager _returnvalue)
  (CallFunction|Reset))

(event EventTakeDamage
  (params (Damage :type Float%20%28double-precision%29) (GaugeGain :type Float%20%28double-precision%29))
  (bind _returnvalue (Transformation|GetActorLocation))
  (bind _ui_offset (Variables|Default|GetUI%20Offset))
  ;[0.1406 0.01245 0.0154 0.85] Take Damage
  (Variables|Stats|SetHealth (- (Variables|Stats|GetHealth) Damage))
  (bind _asbp_player (Utilities|Casting|CastToBP_Player (Game|GetPlayerCharacter 0)))
  (Default|GainGaugePoints _asbp_player GaugeGain)
  ;[1 0.3061 0.7206] UI Damage text
  (bind _returnvalue_2 (Game|SpawnActorfromClass "/Game/UI/FX/BP_DamageText.BP_DamageText_C" (Math|Transform|MakeTransform (Math|Vector|MakeVector (Math|Random|RandomFloatinRange (- (.x _returnvalue) _ui_offset) (+ (.x _returnvalue) _ui_offset)) (Math|Random|RandomFloatinRange (- (.y _returnvalue) _ui_offset) (+ (.y _returnvalue) _ui_offset)) (.z _returnvalue)) "0, 0, 0" "1.000000,1.000000,1.000000") "Undefined" "MultiplyWithRoot" 0 0))
  (bind _aswbp_uidamage (Utilities|Casting|CastToWBP_UIDamage (UserInterface|GetWidget (Variables|/Game/UI/FX/BP_DamageText.BP_DamageText_C|GetWBP_DamageWidget _returnvalue_2))))
  (Variables|/Game/UI/FX/WBP_UIDamage.WBP_UIDamage_C|SetDamage _aswbp_uidamage (Utilities|Text|ToText(Float) Damage "HalfToEven"))
  ;[0.07421 0.002732 0.002428] Game feel
  (Camera|PlayWorldCameraShake "/Game/FX/Effects/Camera/CS_EnemyTakeDamage.CS_EnemyTakeDamage_C" (Transformation|GetActorLocation) 0.0 1e+05 0.0)
  (Niagara|SpawnSystematLocation "/Game/FX/Effects/NS_Impact.NS_Impact" (.location (Transformation|GetActorTransform)))
  (CallFunction|StartHitStop 0.05))

(fn ConstructionScript)

(fn StartHitStop
  (params (Time :type Float%20%28single-precision%29))
  (Variables|Default|SetCustomTimeDilation 0.0)
  (Utilities|Time|SetTimerbyFunctionName 0 "EndHitStop" Time))

(fn EndHitStop
  (Variables|Default|SetCustomTimeDilation 1.0))

(fn Reset
  (Variables|Stats|SetHealth (Variables|Stats|GetMaxHealth))
  (Variables|Stats||Speeds|SetSpeed "NewEnumerator1")
  (Utilities|Array|RemoveItem (Variables|/Game/Enemies/Parent/BP_EnemiesManager.BP_EnemiesManager_C|GetEnemies_dead (Variables|Default|GetManager)) self)
  (Utilities|Array|Add (Variables|/Game/Enemies/Parent/BP_EnemiesManager.BP_EnemiesManager_C|GetEnemies_allive (Variables|Default|GetManager)) self))

(fn GetIdealRange
  (return (Variables|Stats||Ranges|GetAttack%20Range) (Variables|Stats||Ranges|GetDefend%20Range)))

(fn GetPatrolRoute
  (return (Variables|AI|GetPatrolRoute)))

(fn SetMovementSpeed
  (params (Speed :type E_MovementSpeed%20Enum :default "NewEnumerator0"))
  (bind _output_get (Variables|/Script/Engine.CharacterMovementComponent|SetMaxWalkSpeed (Variables|Character|GetCharacterMovement) (Utilities|Select :Index Speed :NewEnumerator0 (Variables|STats||Speeds|GetIdleSpeed) :NewEnumerator1 (Variables|STats||Speeds|GetWalkSpeed) :NewEnumerator2 (Variables|STats||Speeds|GetSemi-%20SprintSpeed) :NewEnumerator3 (Variables|STats||Speeds|GetSprintSpeed))))
  (return _output_get))