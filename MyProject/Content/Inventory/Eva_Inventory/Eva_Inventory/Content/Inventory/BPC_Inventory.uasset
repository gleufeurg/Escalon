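; Inventory component for the third-person character that picks up items into separate Skill, Ring and Weapon inventories, each with its own capacity.
; The item's Type in DT_Item selects the array, count, limit and matching wrap box in the character's inventory widget.
; A successful pickup increments the count, stores the row name, updates the UI and destroys the pickup actor with a sound, while a full category only plays a warning sound.
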(fn AddItemtoInventory
  (params (New%20Item%20Row%20Name :type Name) (PickupItem :type Actor%20Object%20Reference))
  ;[0.4983 0.3125 1 0.55] Pickable check
  ; All items have a name, so if a collider doesn't have one, it can not be picked
  (if (!= New%20Item%20Row%20Name "")
    ;[0.717 0.2545 1 0.85] Check if Is Array Full ?
    (bind _is_array_full_ (CallFunction|CheckArraySize New%20Item%20Row%20Name))
    (if _is_array_full_
      (Audio|PlaySound2D "/Game/SFX/Sounds/SC_InventoryFull.SC_InventoryFull" 1.0 1.0 0.0 0 0)
      (else
        (CallFunction|SetItemArraySize New%20Item%20Row%20Name)
        ;[0.5776 0.2122 0.9473] For now Inventories Arrays are pretty much useless
        ; But it serve as memory for every Items
        (Utilities|Array|Add (Variables|Inventories|GetInventory) "")
        (Utilities|Array|Add (CallFunction|GetItemCorrespondingInventory New%20Item%20Row%20Name) New%20Item%20Row%20Name)
        (bind _asbp_third_person_character (Utilities|Casting|CastToBP_ThirdPersonCharacter (Components|GetOwner)))
        (Default|AddItemtoUIInventory (Variables|/Game/ThirdPerson/Blueprints/BP_ThirdPersonCharacter.BP_ThirdPersonCharacter_C|GetWB_Inventory _asbp_third_person_character) (CallFunction|GetItemCorrectUIInventory New%20Item%20Row%20Name) New%20Item%20Row%20Name)
        (Actor|DestroyActor PickupItem)
        (Audio|PlaySound2D "/Game/SFX/Sounds/SC_Pickup.SC_Pickup" 1.0 1.0 0.0 0 0)))))

(fn GetItemCorrespondingInventory
  (params (Item%20Row%20Name :type Name))
  (bind _returnvalue (Utilities|GetDataTableRow "/Game/Inventory/DT_Item.DT_Item" Item%20Row%20Name)
    (:then
      (switch Utilities|FlowControl|Switch|SwitchonE_ItemType (.type _returnvalue)
        (:NewEnumerator0
          (return (Variables|Inventories|GetSkill%20Inventory)))
        (:NewEnumerator1
          (return (Variables|Inventories|GetRing%20Inventory)))
        (:NewEnumerator2
          (return (Variables|Inventories|GetWeapon%20Inventory)))))))

(fn GetItemCorrectUIInventory
  (params (Item%20Row%20Name :type Name))
  (bind _returnvalue (Utilities|GetDataTableRow "/Game/Inventory/DT_Item.DT_Item" Item%20Row%20Name)
    (:then
      (switch Utilities|FlowControl|Switch|SwitchonE_ItemType (.type _returnvalue)
        (:NewEnumerator0
          (bind _asbp_third_person_character (Utilities|Casting|CastToBP_ThirdPersonCharacter (Components|GetOwner)))
          (return (Variables|/Game/UI/Inventory/WB_Inventory.WB_Inventory_C|GetSkill_WrapBox (Variables|/Game/ThirdPerson/Blueprints/BP_ThirdPersonCharacter.BP_ThirdPersonCharacter_C|GetWB_Inventory _asbp_third_person_character))))
        (:NewEnumerator1
          (bind _asbp_third_person_character_2 (Utilities|Casting|CastToBP_ThirdPersonCharacter (Components|GetOwner)))
          (return (Variables|/Game/UI/Inventory/WB_Inventory.WB_Inventory_C|GetRing_WrapBox (Variables|/Game/ThirdPerson/Blueprints/BP_ThirdPersonCharacter.BP_ThirdPersonCharacter_C|GetWB_Inventory _asbp_third_person_character_2))))
        (:NewEnumerator2
          (bind _asbp_third_person_character_3 (Utilities|Casting|CastToBP_ThirdPersonCharacter (Components|GetOwner)))
          (return (Variables|/Game/UI/Inventory/WB_Inventory.WB_Inventory_C|GetWeapon_WrapBox (Variables|/Game/ThirdPerson/Blueprints/BP_ThirdPersonCharacter.BP_ThirdPersonCharacter_C|GetWB_Inventory _asbp_third_person_character_3))))))))

(fn GetMaxItemArray
  (params (New%20Item%20Row%20Name :type Name))
  (bind _returnvalue (Utilities|GetDataTableRow "/Game/Inventory/DT_Item.DT_Item" New%20Item%20Row%20Name)
    (:then
      (switch Utilities|FlowControl|Switch|SwitchonE_ItemType (.type _returnvalue)
        (:NewEnumerator0
          (return (Variables|Inventories|GetMaxSkill)))
        (:NewEnumerator1
          (return (Variables|Inventories|GetMaxRing)))
        (:NewEnumerator2
          (return (Variables|Inventories|GetMaxWeapon)))))))

(fn GetCurrentIteminArray
  (params (New%20Item%20Row%20Name :type Name))
  (bind _returnvalue (Utilities|GetDataTableRow "/Game/Inventory/DT_Item.DT_Item" New%20Item%20Row%20Name)
    (:then
      (switch Utilities|FlowControl|Switch|SwitchonE_ItemType (.type _returnvalue)
        (:NewEnumerator0
          (return (Variables|Inventories|GetCurrentSkillNum)))
        (:NewEnumerator1
          (return (Variables|Inventories|GetCurrentRingNum)))
        (:NewEnumerator2
          (return (Variables|Inventories|GetCurrentWeaponNum)))))))

(fn SetItemArraySize
  (params (New%20Item%20Row%20Name :type Name))
  (bind _current_item_in_array (CallFunction|GetCurrentIteminArray New%20Item%20Row%20Name))
  (bind _returnvalue (+ _current_item_in_array 1))
  (bind _returnvalue_2 (Utilities|GetDataTableRow "/Game/Inventory/DT_Item.DT_Item" New%20Item%20Row%20Name)
    (:then
      (switch Utilities|FlowControl|Switch|SwitchonE_ItemType (.type _returnvalue_2)
        (:NewEnumerator0
          (Variables|Inventories|SetCurrentSkillNum _returnvalue))
        (:NewEnumerator1
          (Variables|Inventories|SetCurrentRingNum _returnvalue))
        (:NewEnumerator2
          (Variables|Inventories|SetCurrentWeaponNum _returnvalue))))))

(fn CheckArraySize
  (params (New%20Item%20Row%20Name :type Name))
  ;[0.0137 0.7529 0.4179] Check Array length
  (if (>= (- (CallFunction|GetMaxItemArray New%20Item%20Row%20Name) 1) (CallFunction|GetCurrentIteminArray New%20Item%20Row%20Name))
    (return false)
    (else
      (return true))))