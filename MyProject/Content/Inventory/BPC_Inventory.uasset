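; BPC_Inventory is an inventory component on the player character that handles picked-up items.
; AddItemToInventory ignores unnamed colliders, then casts the owner to BP_ThirdPersonCharacter and calls its inventory widget to add the item to the UI.
; GetItemCorrespondingArray maps a data-table row name (Skill, Weapon or Ring) to the matching inventory array, printing a warning when no name matches.
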(fn AddItemtoInventory
  (params (New%20Item%20Name :type Name))
  ;[0.4983 0.3125 1 0.55] Pickable check
  ; All items have a name, so if a collider doesn't have one, it can not be picked
  (if (!= New%20Item%20Name "")
    (bind _asbp_third_person_character (Utilities|Casting|CastToBP_ThirdPersonCharacter (Components|GetOwner)))
    (Default|AddItemtoUIInventory (Variables|/Game/ThirdPerson/Blueprints/BP_ThirdPersonCharacter.BP_ThirdPersonCharacter_C|GetWB_Inventory _asbp_third_person_character))))

(fn GetItemCorrespondingArray
  (params (Item%20Name :type Name))
  (if (== Item%20Name "Skill")
    (return (Variables|Default|GetSkill%20Inventory))
    (elif (== Item%20Name "Weapon")
      (return (Variables|Default|GetWeapon%20Inventory))
      (elif (== Item%20Name "Ring")
        (return (Variables|Default|GetRing%20Inventory))
        (else
          (Development|PrintString "Item don't match any array name 
Try to look on the Raw Name Comment 
Does the raw name has been changed lately ? 
The Item data table raw name has to be the exact same as those" true true "(R=1.000000,G=0.864302,B=0.005986,A=1.000000)"))))))